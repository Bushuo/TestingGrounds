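; NPC AI controller for guard characters, driving patrol and focus behaviour through a behavior tree.
; On begin play it loads the PatrolData blackboard, runs GuardBehavior and caches the blackboard component.
; AI perception updates feed the FocusActor key, setting it when a non-Guard actor is sensed and clearing it when that actor is lost.
; Actors tagged Guard are ignored, so guards do not focus on each other.
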(event OnTargetPerceptionUpdated(AIPerception)
  (params (Actor :type Actor%20Object%20Reference) (Stimulus :type AI%20Stimulus%20Structure))
  (CallFunction|UpdateFocusActorKey Actor Actor Stimulus))

(event EventBeginPlay
  (bind _blackboardcomponent (Class|AIController|UseBlackboard "/Game/Dynamic/Character/AI/PatrolData.PatrolData"))
  (AI|RunBehaviorTree "/Game/Dynamic/Character/AI/GuardBehavior.GuardBehavior")
  (Variables|Default|SetBlackboardComp _blackboardcomponent))

(fn ConstructionScript)

(fn UpdateFocusActorKey
  (params (Actor :type Actor%20Object%20Reference) (ObjectValue :type Object%20Object%20Reference) (AIStimulus :type AI%20Stimulus%20Structure%20%28by%20ref%29))
  (bind _focusactor (Variables|Default|GetFocusActor))
  (bind _blackboardcomp (Variables|Default|GetBlackboardComp))
  (if (not (Actor|ActorHasTag Actor "Guard"))
    (if (.bSuccessfullySensed (Utilities|Struct|BreakAIStimulus AIStimulus))
      (AI|Components|Blackboard|SetValueasObject _blackboardcomp _focusactor ObjectValue)
      (else
        (AI|Components|Blackboard|ClearValue _blackboardcomp _focusactor)))))