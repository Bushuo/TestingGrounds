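; TileBP is a terrain tile for an endless level built piece by piece through the InfiniteTerrain game mode.
; Its end barrier starts solid and red, then turns passable and green while the player is inside LockVolume.
; Leaving LockVolume relocks the barrier and asks the game mode to spawn the next tile.
; GetAttachLocation exposes the AttachPoint transform, and the tile destroys itself when the player enters GarbadgeVolume.
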(event OnComponentEndOverlap(LockVolume)
  (params (OverlappedComponent :type Primitive%20Component%20Object%20Reference) (OtherActor :type Actor%20Object%20Reference) (OtherComp :type Primitive%20Component%20Object%20Reference) (OtherBodyIndex :type Integer))
  (if (== OtherActor (Game|Player|GetPlayerPawn 0))
    (CallFunction|LockLevel)
    (bind _asinfinite_terrain (Utilities|Casting|CastToInfiniteTerrain (Game|GetGameMode)))
    (Default|SpawnNextTile _asinfinite_terrain)))

(event OnComponentBeginOverlap(LockVolume)
  (params (OverlappedComponent :type Primitive%20Component%20Object%20Reference) (OtherActor :type Actor%20Object%20Reference) (OtherComp :type Primitive%20Component%20Object%20Reference) (OtherBodyIndex :type Integer) (bFromSweep :type Boolean) (SweepResult :type Hit%20Result%20Structure%20%28by%20ref%29))
  (if (== OtherActor (Game|Player|GetPlayerPawn 0))
    (CallFunction|UnlockLevel)))

(event OnComponentBeginOverlap(GarbadgeVolume)
  (params (OverlappedComponent :type Primitive%20Component%20Object%20Reference) (OtherActor :type Actor%20Object%20Reference) (OtherComp :type Primitive%20Component%20Object%20Reference) (OtherBodyIndex :type Integer) (bFromSweep :type Boolean) (SweepResult :type Hit%20Result%20Structure%20%28by%20ref%29))
  (if (== OtherActor (Game|Player|GetPlayerPawn 0))
    (Actor|DestroyActor)))

(event EventBeginPlay
  (CallFunction|LockLevel))

(fn ConstructionScript)

(fn GetAttachLocation
  (return (Transformation|GetWorldTransform (Variables|Default|GetAttachPoint))))

(fn UnlockLevel
  (Collision|SetCollisionEnabled (Variables|Default|GetLevelEndBarrier) "NoCollision")
  (Rendering|Material|SetMaterial (Variables|Default|GetLevelEndBarrier) 0 "/Game/Dynamic/Terrain/GreenEmissive.GreenEmissive"))

(fn LockLevel
  (Collision|SetCollisionEnabled (Variables|Default|GetLevelEndBarrier) "QueryAndPhysics")
  (Rendering|Material|SetMaterial (Variables|Default|GetLevelEndBarrier) 0 "/Game/Dynamic/Terrain/RedEmissive.RedEmissive"))