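; AI controller for guard NPCs that runs the GuardBehavior behavior tree on the PatrolData blackboard.
; AI perception stores sensed actors without the Guard tag in the blackboard's FocusActor key and clears the key when sensing is lost.
; Every tick it sets the possessed TPCharacter's Focused and Shooting flags to whether the controller has a valid focus actor.
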(event OnTargetPerceptionUpdated(AIPerception)
  (params (Actor :type Actor%20Object%20Reference) (Stimulus :type AI%20Stimulus%20Structure))
  (if (not (Actor|ActorHasTag Actor "Guard"))
    (if (.bSuccessfullySensed (Utilities|Struct|BreakAIStimulus Stimulus))
      (AI|Components|Blackboard|SetValueasObject (Variables|Default|GetBlackboardComp) (Variables|Default|GetFocusActor) Actor)
      (else
        (AI|Components|Blackboard|ClearValue (Variables|Default|GetBlackboardComp) (Variables|Default|GetFocusActor))))))

(event EventBeginPlay
  (bind _blackboardcomponent (Class|AIController|UseBlackboard "/Game/Dynamic/NPC/AI/PatrolData.PatrolData"))
  (AI|RunBehaviorTree "/Game/Dynamic/NPC/AI/GuardBehavior.GuardBehavior")
  (Variables|Default|SetBlackboardComp _blackboardcomponent))

(event EventTick
  (params (DeltaSeconds :type Float%20%28single-precision%29))
  (bind _astpcharacter (Utilities|Casting|CastToTPCharacter (Pawn|GetControlledPawn)))
  (bind _output_get (Variables|/Game/Dynamic/NPC/Behaviour/TPCharacter.TPCharacter_C|SetFocused _astpcharacter (Utilities|IsValid (Class|AIController|GetFocusActor))))
  (Variables|/Game/Dynamic/NPC/Behaviour/TPCharacter.TPCharacter_C|SetShooting _astpcharacter _output_get))

(fn ConstructionScript)